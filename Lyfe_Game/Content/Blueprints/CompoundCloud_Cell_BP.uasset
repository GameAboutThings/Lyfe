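; Compound cloud Blueprint for a cell setting, representing one compound type: CO2, O2, amino acid, glucose or lipid.
; Actor overlap events pass straight through to BeginOverlap and EndOverlap, which are defined outside this graph.
; GenerateCloudColor maps the type to a tint, which ApplyCloudColor writes to each particle component through a dynamic material instance's Color parameter.
; Invalid components get a debug marker; nothing here calls ApplyCloudColor.
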(event EventBeginPlay)

(event EventTick
  (params (DeltaSeconds :type Float%20%28single-precision%29)))

(event Collision|EventActorBeginOverlap
  (params (OtherActor :type Actor%20Object%20Reference))
  (Class|CompoundCloudCell|BeginOverlap OtherActor))

(event Collision|EventActorEndOverlap
  (params (OtherActor :type Actor%20Object%20Reference))
  (Class|CompoundCloudCell|EndOverlap OtherActor))

(fn ConstructionScript)

(fn GenerateCloudColor
  (bind _returnvalue (Class|CompoundCloudCell|GetType))
  (switch Utilities|FlowControl|Switch|SwitchonECompound _returnvalue
    (:ECO2
      (return (Math|Color|MakeColor 0.6 1.0 0.8 0.0)))
    (:EO2
      (return (Math|Color|MakeColor 1.0 0.6 0.4 0.0)))
    (:EAminoAcid
      (return (Math|Color|MakeColor 0.4 1.0 0.6 0.0)))
    (:EGlucose
      (return (Math|Color|MakeColor 1.0 1.0 1.0 0.0)))
    (:ELipid
      (return (Math|Color|MakeColor 1.0 1.0 0.6 0.0)))))

(fn ApplyCloudColor
  (bind _returnvalue (Class|CompoundCloudCell|GetParticleComponents))
  (for (_array_element _array_index) _returnvalue
    (Utilities|IsValid _array_element
      (:Is%20Valid
        (bind _returnvalue_2 (Class|CompoundParticleComponentCell|GetParticleSystem _array_element))
        (bind _returnvalue_3 (Rendering|Material|CreateDynamicMaterialInstance (Rendering|Material|GetMaterial _returnvalue_2 0) :!class /Script/Engine.KismetMaterialLibrary))
        (bind _color (CallFunction|GenerateCloudColor))
        (Rendering|Material|SetVectorParameterValue _returnvalue_3 "Color" _color :!class /Script/Engine.MaterialInstanceDynamic)
        (Rendering|Material|SetMaterial _returnvalue_2 0 _returnvalue_3))
      (:Is%20Not%20Valid
        (Rendering|Debug|DrawDebugString (Math|Conversions|ToVector(Vector2D) (Math|Vector2D|MakeVector2D (Math|Conversions|ToFloat(Integer) _array_index) 0.0) 1.0) "XX" 0 "(R=1.000000,G=0.000000,B=0.000000,A=1.000000)" 6e+01)))))