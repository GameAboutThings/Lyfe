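; Single-celled player character Blueprint that forwards movement and camera-style zoom input to functions defined outside this graph.
; On BeginPlay it assigns the Ball component as PlayerMesh and turns on its overlap events.
; MoveForward and MoveRight axes feed SetForwardMotion and SetRightMotion, while mouse wheel presses pass a signed step to Zoom.
; The actor overlap event and construction script are empty.
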(event EventBeginPlay
  (bind _output_get (Variables|Default|SetplayerMesh (Variables|Default|Getball)))
  (Variables|/Script/Engine.PrimitiveComponent|SetbGenerateOverlapEvents _output_get true))

(event Collision|EventActorBeginOverlap
  (params (OtherActor :type Actor%20Object%20Reference)))

(event Input|AxisEvents|InputAxisMoveForward
  (params (AxisValue :type Float%20%28single-precision%29))
  (Class|CharacterSingleCelled|SetForwardMotion AxisValue))

(event Input|AxisEvents|InputAxisMoveRight
  (params (AxisValue :type Float%20%28single-precision%29))
  (Class|CharacterSingleCelled|SetRightMotion AxisValue))

(event Input|MouseEvents|MouseWheelDown
  (params (Key :type Key%20Structure))
  (:Pressed
    (Variables|Default|Setzoom_0 1.0)
    (Class|CharacterSingleCelled|Zoom (Variables|Default|Getzoom_0))))

(event Input|MouseEvents|MouseWheelUp
  (params (Key :type Key%20Structure))
  (:Pressed
    (Variables|Default|Setzoom_0 -1.0)
    (Class|CharacterSingleCelled|Zoom (Variables|Default|Getzoom_0))))

(fn ConstructionScript)