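; Base Blueprint for an editor cell, shown as a ball node with four directional arrows (left, down, up, right).
; The construction script runs SetMeshes to assign the ball and arrow meshes and enlarge the arrows uniformly.
; SetMaterials then applies a dynamic instance of the editor node material to the ball only.
; The event graph is empty, so this Blueprint only handles visual setup.
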(event EventBeginPlay)

(event Collision|EventActorBeginOverlap
  (params (OtherActor :type Actor%20Object%20Reference)))

(event EventTick
  (params (DeltaSeconds :type Float%20%28single-precision%29)))

(fn ConstructionScript
  (CallFunction|SetMeshes)
  (CallFunction|SetMaterials))

(fn SetMaterials
  (Utilities|FlowControl|Sequence
    (:then_0
      ;[1 1 1] Nodes
      (bind _returnvalue (Rendering|Material|CreateDynamicMaterialInstance "/Game/Materials/M_Editor_Node.M_Editor_Node" :!class /Script/Engine.KismetMaterialLibrary))
      (bind _returnvalue_2 (Class|CellEditorNodeComponent|GetMesh (Variables|Default|GetbaseNode)))
      (Rendering|Material|SetMaterial _returnvalue_2 0 _returnvalue))))

(fn SetMeshes
  (bind _arrowleft (Variables|Default|GetarrowLeft))
  (bind _arrowdown (Variables|Default|GetarrowDown))
  (bind _arrowup (Variables|Default|GetarrowUp))
  (bind _arrowright (Variables|Default|GetarrowRight))
  (Variables|Default|SetRelativeScale "5.000000,5.000000,5.000000")
  (Utilities|FlowControl|Sequence
    (:then_0
      (bind _returnvalue (Class|CellEditorNodeComponent|GetMesh (Variables|Default|GetbaseNode)))
      (Components|StaticMesh|SetStaticMesh _returnvalue "/Game/Meshes/ball.ball"))
    (:then_1
      (bind _returnvalue_2 (Class|CellEditorArrowComponent|GetMeshComponent _arrowleft))
      (Components|StaticMesh|SetStaticMesh _returnvalue_2 "/Game/Meshes/Arrow.Arrow")
      (Transformation|SetRelativeScale3D _arrowleft (Variables|Default|GetRelativeScale)))
    (:then_2
      (bind _returnvalue_3 (Class|CellEditorArrowComponent|GetMeshComponent _arrowdown))
      (Components|StaticMesh|SetStaticMesh _returnvalue_3 "/Game/Meshes/Arrow.Arrow")
      (Transformation|SetRelativeScale3D _arrowdown (Variables|Default|GetRelativeScale)))
    (:then_3
      (bind _returnvalue_4 (Class|CellEditorArrowComponent|GetMeshComponent _arrowup))
      (Components|StaticMesh|SetStaticMesh _returnvalue_4 "/Game/Meshes/Arrow.Arrow")
      (Transformation|SetRelativeScale3D _arrowup (Variables|Default|GetRelativeScale)))
    (:then_4
      (bind _returnvalue_5 (Class|CellEditorArrowComponent|GetMeshComponent _arrowright))
      (Components|StaticMesh|SetStaticMesh _returnvalue_5 "/Game/Meshes/Arrow.Arrow")
      (Transformation|SetRelativeScale3D _arrowright (Variables|Default|GetRelativeScale)))))