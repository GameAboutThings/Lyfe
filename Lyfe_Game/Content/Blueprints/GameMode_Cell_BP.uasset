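; Game mode Blueprint for the cell part of the game that sets up the HUD and mouse on BeginPlay.
; It creates and shows the cell HUD widget and enables the cursor.
; When disableWASDInput is set, it calls SetIgnoreMoveInput with false, centers the mouse, sets LowCompound to carbon and starts the low-compound cycle.
; Tick is empty, and the UpdateLowCompound and DisableWASDInput calls are unconnected.
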(event EventBeginPlay
  (bind _returnvalue (Game|GetPlayerController 0))
  (bind _returnvalue_2 (Viewport|GetViewportSize))
  (bind (_x _y) (Math|Vector2D|BreakVector2D _returnvalue_2))
  (bind _returnvalue_3 (UserInterface|CreateWidget "/Game/Blueprints/HUD_Cell_BP.HUD_Cell_BP_C" (Game|GetPlayerController 0)))
  (UserInterface|Viewport|AddtoViewport _returnvalue_3 0)
  (Variables|/Script/Engine.PlayerController|SetbShowMouseCursor _returnvalue true)
  (if (stale _returnvalue)
    (Input|SetIgnoreMoveInput _returnvalue false)
    (Class|PlayerController|SetMouseLocation _returnvalue (Math|Float|Truncate (/ _x 2.0)) (Math|Float|Truncate (/ _y 2.0)))
    (Variables|Default|SetlowCompound "carbon")
    (Class|GameModeCell|StartLowCompoundCycle)))

(event EventTick
  (params (DeltaSeconds :type Float%20%28single-precision%29)))

(fn ConstructionScript)